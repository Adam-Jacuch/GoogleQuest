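; BP_GameManager is an actor that tracks an ordered button-press sequence and handles losing the game.
; BeginPlay hides the cursor and sets game-only input.
; CheckButton compares a pressed number against ExpectedButton, and AdvanceButton increments that expected value.
; LoseGame shows the WBP_Lose widget, reveals the cursor and switches to UI-only input.
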(event `self.ReceiveBeginPlay`
  (bind _returnvalue (`GameplayStatics.GetPlayerController` 0))
  (set `PlayerController.bShowMouseCursor` false _returnvalue)
  (`WidgetBlueprintLibrary.SetInputMode_GameOnly` _returnvalue))

(event `LoseGame`
  (bind _returnvalue (`GameplayStatics.GetPlayerController` 0))
  (bind _returnvalue_2 (`|CreateWidget` "/Game/CustomBP/WBP_Lose.WBP_Lose_C"))
  (`UserWidget.AddToViewport` _returnvalue_2 0)
  (set `PlayerController.bShowMouseCursor` true _returnvalue)
  (`WidgetBlueprintLibrary.SetInputMode_UIOnlyEx` _returnvalue null))

(fn `AdvanceButton`
  (set `self.ExpectedButton` (+ (`self.ExpectedButton`) 1)))

(fn `CheckButton`
  (params (PressedNumber :type Integer))
  (returns (Correct :type Boolean))
  (return (== PressedNumber (`self.ExpectedButton`))))

(fn `UserConstructionScript`)
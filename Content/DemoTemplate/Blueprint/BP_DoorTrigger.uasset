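; BP_DoorTrigger is an overlap trigger in a numbered button sequence, checked against BP_GameManager.
; A correct overlap marks it used, advances the sequence, enables physics on selected targets and launches mannequins with an impulse.
; The mannequin loop nests inside the target loop, and the fifth button's WinGame call sits inside both.
; A wrong overlap loses the game unless the trigger was already used.
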(event `self.ReceiveBeginPlay`
  (bind _returnvalue (`PrimitiveComponent.CreateDynamicMaterialInstance` (`self.SM_CircularGlow`) 0 null "None"))
  (set `self.MID_LIght` _returnvalue))

(event `self.ReceiveActorBeginOverlap`
  (params (OtherActor :type "Actor Object Reference"))
  (bind _returnvalue (`GameplayStatics.GetActorOfClass` "/Game/CustomBP/BP_GameManager.BP_GameManager_C"))
  (bind _asbp_game_manager (cast `/Game/CustomBP/BP_GameManager` _returnvalue))
  (bind _correct (`/Game/CustomBP/BP_GameManager.CheckButton` _asbp_game_manager (`self.ButtonNumber`)))
  (if _correct
    (set `self.Used` true)
    (`/Game/CustomBP/BP_GameManager.AdvanceButton` _asbp_game_manager)
    (for _array_element (`self.TargetSelection`)
      (`PrimitiveComponent.SetSimulatePhysics` (`StaticMeshActor.StaticMeshComponent` _array_element) true)
      (for _array_element_2 (`self.MannequinTargets`)
        (bind _skeletalmeshcomponent (`SkeletalMeshActor.SkeletalMeshComponent` _array_element_2))
        (`PrimitiveComponent.SetSimulatePhysics` _skeletalmeshcomponent true)
        (`PrimitiveComponent.WakeRigidBody` _skeletalmeshcomponent "None")
        (`PrimitiveComponent.AddImpulse` _skeletalmeshcomponent (1200.0 600.0 2400.0) "None" false)
        (if (== (`self.ButtonNumber`) 5)
          (`/Game/CustomBP/BP_GameManager.WinGame` _asbp_game_manager))))
    (elif (not (`self.Used`))
      (`/Game/CustomBP/BP_GameManager.LoseGame` _asbp_game_manager))))

(fn `UserConstructionScript`)